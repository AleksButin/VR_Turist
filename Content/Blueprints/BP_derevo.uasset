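; BP_derevo is a choppable tree that breaks down into a stump and branches when hit with an axe.
; Each capsule overlap with BP_axe plays a chop sound and increments the Udar hit counter.
; From the third hit, it hides the tree mesh, disables its collision and reveals a rotten stump mesh.
; A DoOnce then spawns a batch of BP_vetka branch actors at the Scene component's location, only once.
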(event `self.Capsule.OnComponentBeginOverlap`
  (params (OverlappedComponent :type "PrimitiveComponent Object Reference") (OtherActor :type "Actor Object Reference") (OtherComp :type "PrimitiveComponent Object Reference") (OtherBodyIndex :type Integer) (bFromSweep :type Boolean) (SweepResult :type "HitResult Structure (by ref)"))
  (cast `/Game/Blueprints/BP_axe` OtherActor)
  (`GameplayStatics.PlaySoundAtLocation` "/Game/Sound/derevo_zvuk2_Cue.derevo_zvuk2_Cue" (`SceneComponent.K2_GetComponentLocation` (`self.StaticMeshComponent`)) (struct) 1.0 1.0 0.0 null null null null)
  (bind _output_get (set `self.Udar` (+ (`self.Udar`) 1)))
  (if (>= _output_get 3)
    (`SceneComponent.SetVisibility` (`self.StaticMeshComponent`) false false)
    (`SceneComponent.SetVisibility` (`self.S_Rotten_Tree_Stump_wjzueccs_lod3_Var1`) true false)
    (`PrimitiveComponent.SetCollisionProfileName` (`self.StaticMeshComponent`) "NoCollision" true)
    (`/Engine/EditorBlueprintResources/StandardMacros.DoOnce` false
      (:`Completed`
        (for _ (range 5)
          (`|SpawnActorFromClass` "/Game/Blueprints/BP_vetka.BP_vetka_C" (`KismetMathLibrary.MakeTransform` (`SceneComponent.K2_GetComponentLocation` (`self.Scene`))) "Undefined" "MultiplyWithRoot" null null))))))

(fn `UserConstructionScript`)